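; BP_WebcamBillboard is an actor that relays webcam video frames to a billboard widget.
; On each new frame it passes VideoTexture to WDWebcamBillboard, if valid, and the C key calls ChangeOperation, which is defined outside this graph.
; BeginPlay enables input and creates a dynamic M_Webcam material on the Billboard component.
; The nodes that would set that material's texture parameter or reassign it are disconnected, so frames reach only the widget.
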(event `self.ReceiveBeginPlay`
  (`self.EnableInput` (`GameplayStatics.GetPlayerController` 0))
  (bind _returnvalue (`PrimitiveComponent.CreateDynamicMaterialInstance` (`self.Billboard`) 0 "/Game/Materials/M_Webcam.M_Webcam"))
  (set `self.DynamicMaterial` _returnvalue))

(event `self.OnNextVideoFrame`
  (bind _wdwebcambillboard (`self.WDWebcamBillboard`))
  (`/Engine/EditorBlueprintResources/StandardMacros.IsValid` _wdwebcambillboard
    (:`Is Valid`
      (`/Game/UI/WD_WebcamBillboard.UpdateVideoFrame` _wdwebcambillboard (`self.VideoTexture`)))))

(event `Key|C`
  (params (Key :type "Key Structure"))
  (:`Pressed`
    (`self.ChangeOperation`)))

(fn `UserConstructionScript`)